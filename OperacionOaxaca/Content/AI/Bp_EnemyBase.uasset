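; Base enemy Blueprint that chases the player for melee attacks and fires a gun at its AI focus actor.
; Chase moves to the player, triggers a punch montage and repeats after a delay; Attack broadcasts OnAttackEnd when the montage completes or is interrupted.
; Tick fires every frame while a focus exists, tracing toward the target's randomly rotated world position.
; Shots play muzzle Niagara and sound, spawning a trail on hits, without applying damage.
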(event Custom|Chase
  (AI|AIMoveTo self "10000.000000,20000000000000000000.000000,0.010000" (Game|GetPlayerCharacter 0) 5.0 false
    (:OnSuccess
      (CallFunction|Attack)
      (Utilities|FlowControl|Delay 2.0)
      (CallFunction|Chase))))

(event Custom|Attack
  (Animation|Montage|PlayMontage (Variables|Character|GetMesh) "/Game/AI/Anim/H2H_PunchCombo02_Montage.H2H_PunchCombo02_Montage"
    (:OnCompleted
      _)
    (:OnInterrupted
      _))
  (Default|CallOnAttackEnd))

(event Custom|FireBullet
  (bind _self self)
  (bind _returnvalue (AI|GetAIController _self))
  (bind _returnvalue_2 (Class|AIController|GetFocusActor _returnvalue))
  (Utilities|IsValid _returnvalue_2
    (:Is%20Valid
      (bind (_outhit _returnvalue_3) (Collision|LineTraceByChannel (Transformation|GetWorldLocation (Variables|Default|GetGun)) (Math|Vector|RotateVector (Transformation|GetActorLocation _returnvalue_2) (Math|Rotator|MakeRotator (Math|Random|RandomFloatinRange -2e+01 2e+01) (Math|Random|RandomFloatinRange -2e+01 2e+01) 0.0)) "TraceTypeQuery2" false 0 "None"))
      (Components|Activation|Activate (Variables|Default|GetNiagara) false)
      (Audio|PlaySoundatLocation "/Game/Game/Sounds/Guns/Ak-47_shot.Ak-47_shot" (Transformation|GetActorLocation) "0, 0, 0" 1.0 1.0 0.0 0 0 0 0)
      (if _returnvalue_3
        (Niagara|SpawnSystematLocation "/Game/Game/Particles/NS_BulletTrail.NS_BulletTrail" (.Location (Collision|BreakHitResult _outhit)) (Math|Rotator|MakeRotfromX (.ImpactPoint (Collision|BreakHitResult _outhit))))))))

(event EventBeginPlay)

(event Collision|EventActorBeginOverlap
  (params (OtherActor :type Actor%20Object%20Reference)))

(event EventTick
  (params (DeltaSeconds :type Float%20%28single-precision%29))
  (CallFunction|FireBullet))

(fn ConstructionScript)