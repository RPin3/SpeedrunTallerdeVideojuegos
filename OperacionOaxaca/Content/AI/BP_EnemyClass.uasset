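; Enemy actor Blueprint that shoots at its AI controller's focus actor on every Tick, with no cooldown.
; Each shot line-traces on the Camera channel from the Gun to the focus actor's world location vector, rotated by random pitch and roll for inaccuracy.
; It activates Niagara, plays a sound and spawns an effect at any hit, but applies no damage.
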(event Custom|FireBullet
  (bind _self self)
  (bind _returnvalue (AI|GetAIController _self))
  (bind _returnvalue_2 (Class|AIController|GetFocusActor _returnvalue))
  (Utilities|IsValid _returnvalue_2
    (:Is%20Valid
      (bind (_outhit _returnvalue_3) (Collision|LineTraceByChannel (Transformation|GetWorldLocation (Variables|Default|GetGun)) (Math|Vector|RotateVector (Transformation|GetActorLocation _returnvalue_2) (Math|Rotator|MakeRotator (Math|Random|RandomFloatinRange -2e+01 2e+01) (Math|Random|RandomFloatinRange -2e+01 2e+01) 0.0)) "TraceTypeQuery2" false 0 "None"))
      (Components|Activation|Activate (Variables|Default|GetNiagara) false)
      (Audio|PlaySoundatLocation 0 (Transformation|GetActorLocation) "0, 0, 0" 1.0 1.0 0.0 0 0 0 0)
      (if _returnvalue_3
        (Niagara|SpawnSystematLocation 0 (.Location (Collision|BreakHitResult _outhit)) (Math|Rotator|MakeRotfromX (.ImpactPoint (Collision|BreakHitResult _outhit))))))))

(event EventBeginPlay)

(event Collision|EventActorBeginOverlap
  (params (OtherActor :type Actor%20Object%20Reference)))

(event EventTick
  (params (DeltaSeconds :type Float%20%28single-precision%29))
  (CallFunction|FireBullet))

(fn ConstructionScript)