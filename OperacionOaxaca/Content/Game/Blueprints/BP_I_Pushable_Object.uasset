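; Pushable block actor that reports itself through interaction interface functions as a non-holdable PushableBlock.
; On BeginPlay it measures its height with traces from above and below, then ticks as the player enters or leaves a detection sphere.
; Tick derives manual velocity from flip-flopped location samples, scaling movement sound volume by speed while a downward sphere trace hits.
; UpdatePhysicState toggles physics simulation together with a trace channel's collision response.
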(event OnComponentBeginOverlap(DetectPlayer)
  (params (OverlappedComponent :type Primitive%20Component%20Object%20Reference) (OtherActor :type Actor%20Object%20Reference) (OtherComp :type Primitive%20Component%20Object%20Reference) (OtherBodyIndex :type Integer) (bFromSweep :type Boolean) (SweepResult :type Hit%20Result%20Structure%20%28by%20ref%29))
  ;[1 1 1] Detect Player Pawn
  (if (== OtherActor (Game|Player|GetPlayerPawn 0))
    (Actor|Tick|SetActorTickEnabled true)))

(event OnComponentEndOverlap(DetectPlayer)
  (params (OverlappedComponent :type Primitive%20Component%20Object%20Reference) (OtherActor :type Actor%20Object%20Reference) (OtherComp :type Primitive%20Component%20Object%20Reference) (OtherBodyIndex :type Integer))
  ;[1 1 1] Detect Player Pawn
  (if (== OtherActor (Game|Player|GetPlayerPawn 0))
    (Actor|Tick|SetActorTickEnabled false)))

(event EventTick
  (params (DeltaSeconds :type Float%20%28single-precision%29))
  ;[1 1 1] Tick Event
  (Utilities|CalculateVelocity)
  (CallFunction|UpdateAudioVolume))

(event EventBeginPlay
  ;[1 1 1] Begin Play
  (Audio|Components|Audio|SetSound (Variables|Default|GetSoundFX) (Variables|Default|GetMovement%20Sound))
  (bind _height (CallFunction|FindBoxHeight))
  (bind _output_get (Variables|Default|SetBox%20Height _height))
  (if (== _output_get 0.0)
    (Actor|Tick|SetActorTickEnabled false)
    (else
      (Components|Sphere|SetSphereRadius (Variables|Default|GetDetectPlayer) (Variables|Default|GetDetection%20Player%20Radius) true))))

(fn ConstructionScript
  (Components|StaticMesh|SetStaticMesh (Variables|Default|GetVisual_Mesh) (Variables|Default|GetVisual%20Static%20Mesh)))

(fn UpdatePhysicState
  (params (Stop%20Simulate :type Boolean))
  (if Stop%20Simulate
    (if (Class|SceneComponent|IsAnySimulatingPhysics (Variables|Default|GetCollision))
      (Physics|SetSimulatePhysics (Variables|Default|GetCollision) false)
      (Collision|SetCollisionResponsetoChannel (Variables|Default|GetCollision) "ECC_GameTraceChannel4" "ECR_Block")
      (return true)
      (else
        (return false)))
    (elif (Class|SceneComponent|IsAnySimulatingPhysics (Variables|Default|GetCollision))
      (return false)
      (else
        (Physics|SetSimulatePhysics (Variables|Default|GetCollision) true)
        (Collision|SetCollisionResponsetoChannel (Variables|Default|GetCollision) "ECC_GameTraceChannel4" "ECR_Ignore")
        (return true)))))

(fn FindBoxHeight
  (Utilities|FlowControl|Sequence
    (:then_0
      ;[1 1 1] Up
      (bind (_outhits _returnvalue) (Collision|MultiLineTraceByChannel (+ (Transformation|GetActorLocation) (* (Transformation|GetActorUpVector) (+ (.SphereRadius (Collision|GetComponentBounds (Variables|Default|GetCollision))) 1e+01))) (Transformation|GetActorLocation) "TraceTypeQuery5" false 0 (Variables|Default|GetDraw%20Debug%20Type) false "(R=1.000000,G=0.000000,B=0.000000,A=1.000000)" "(R=0.000000,G=1.000000,B=0.000000,A=1.000000)" 2.0))
      (if _returnvalue
        (if (== (Utilities|Array|Length _outhits) 1)
          (LocalVariables|SetUp%20impact%20 (.ImpactPoint (Collision|BreakHitResult (Utilities|Array|Get(acopy) _outhits))))
          (else
            (bind _array_element (Utilities|Array|ForEachLoopwithBreak _outhits :!label _label)
              (:LoopBody
                (if (== (.HitActor (Collision|BreakHitResult _array_element)) self)
                  (LocalVariables|SetUp%20impact%20 (.ImpactPoint (Collision|BreakHitResult _array_element)))
                  (goto _label Break))))))
        (else
          (return 0.0))))
    (:then_1
      ;[1 1 1] Down
      (bind (_outhits_2 _returnvalue_2) (Collision|MultiLineTraceByChannel (+ (Transformation|GetActorLocation) (* (Transformation|GetActorUpVector) (* (+ (.SphereRadius (Collision|GetComponentBounds (Variables|Default|GetCollision))) 1e+01) -1.0))) (Transformation|GetActorLocation) "TraceTypeQuery5" false 0 (Variables|Default|GetDraw%20Debug%20Type) false "(R=1.000000,G=0.000000,B=0.000000,A=1.000000)" "(R=0.000000,G=1.000000,B=0.000000,A=1.000000)" 2.0))
      (if _returnvalue_2
        (if (== (Utilities|Array|Length _outhits_2) 1)
          (LocalVariables|SetDown%20Impact (.ImpactPoint (Collision|BreakHitResult (Utilities|Array|Get(acopy) _outhits_2))))
          (else
            (bind _array_element_2 (Utilities|Array|ForEachLoopwithBreak _outhits_2 :!label _label_2)
              (:LoopBody
                (if (== (.HitActor (Collision|BreakHitResult _array_element_2)) self)
                  (LocalVariables|SetDown%20Impact (.ImpactPoint (Collision|BreakHitResult _array_element_2)))
                  (goto _label_2 Break))))))
        (else
          (return 0.0))))
    (:then_2
      ;[1 1 1] Return
      (return (- (.z (LocalVariables|GetUp%20impact%20)) (.z (LocalVariables|GetDown%20Impact)))))))

(fn UpdateAudioVolume
  (bind _returnvalue (Collision|SphereTraceByChannel (Transformation|GetActorLocation) (+ (Transformation|GetActorLocation) (* (Math|Vector|VectorGetAbs (Transformation|GetActorUpVector)) (* (/ (Variables|Default|GetBox%20Height) 2.0) -1.15))) 16.0 "TraceTypeQuery1" false 0 (Variables|Default|GetDraw%20Debug%20Type) true "(R=0.000000,G=0.001961,B=0.322917,A=1.000000)" "(R=0.000000,G=1.000000,B=0.717578,A=1.000000)" 0.0))
  (if _returnvalue
    (Audio|Components|Audio|SetVolumeMultiplier (Variables|Default|GetSoundFX) (Math|Float|MapRangeClamped (/ (Math|Vector|VectorLength (Variables|Default|GetVelocity)) (Utilities|Time|GetWorldDeltaSeconds)) 0.0 2e+02 0.0 1.0) :!class /Script/Engine.AudioComponent)
    (else
      (Audio|Components|Audio|SetVolumeMultiplier (Variables|Default|GetSoundFX) 0.0 :!class /Script/Engine.AudioComponent))))

(fn BPIActorStartedInteraction
  (return false))

(fn BPIConfigHoldingOption
  (return false "NewEnumerator0"))

(fn BPIGetInteractionType
  (return "NewEnumerator5"))

(fn BPIGetInteractObjectConfig
  (return false false "" "" 0.0 false false 0))

(fn BPIGetItemtoPickType
  (return "None"))

(fn BPIGetManualVelocity
  (return (Variables|Default|GetVelocity)))

(fn BPIGetObjectCollisionOverlap
  (params (ToIgnore :type Array%20of%20Actor%20Object%20References))
  (return false))

(fn BPIGetObjectTagContainer
  (return "(GameplayTags=((TagName=\"Interaction.PushableBlock\")))"))

(fn BPIGetObjectTraceOrigin
  (return "0, 0, 0"))